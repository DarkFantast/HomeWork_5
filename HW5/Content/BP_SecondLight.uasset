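; BP_SecondLight is an actor that blinks a spot light a set number of times when play begins.
; BeginPlay enters a delay-driven loop that calls LightOff and LightOn in turn, waiting TimeForSecond after each by toggling SpotLight visibility.
; A DoN node caps the repeats at AmountForSecond, so the loop stops after its last LightOff call.
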(event `self.ReceiveBeginPlay`
  (`/Engine/EditorBlueprintResources/StandardMacros.DoOnce` false
    (:`Completed`
      (`self.LightOff` :!label _label)
      (`KismetSystemLibrary.Delay` (`self.TimeForSecond`))
      (`/Engine/EditorBlueprintResources/StandardMacros.Do N` (`KismetMathLibrary.Conv_ByteToInt` (`self.AmountForSecond`))
        (:`Exit`
          (`self.LightOn`)
          (`KismetSystemLibrary.Delay` (`self.TimeForSecond`))
          (goto _label))))))

(fn `LightOff`
  (`SceneComponent.SetVisibility` (`self.SpotLight`) (`self.Off`) false))

(fn `LightOn`
  (`SceneComponent.SetVisibility` (`self.SpotLight`) (`self.On`) false))

(fn `UserConstructionScript`)